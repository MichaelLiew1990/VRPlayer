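; VR pawn for a 180/360 movie player that keeps a video sphere centered on the camera every tick and plays the media sound.
; Setup events swap the sphere's mesh, material and rotation for mono, up-down or left-right layouts in 180 or 360, defaulting to up-down 360.
; A looping timer attaches the widget interaction to the tracked motion controller, preferring the right; triggers and left mouse act as pointer clicks.
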(event `self.ReceiveBeginPlay`
  ;[1 1 1] Play Setting
  (`GameplayStatics.PlaySoundAtLocation` "/Game/Movies/MediaSoundWave.MediaSoundWave")
  (`KismetSystemLibrary.K2_SetTimer` self "CheckMotionController" 1.0 true)
  (bind _outactors (`GameplayStatics.GetAllActorsOfClass` "/Game/_Game/Blueprints/BP_SphereMoviePlayer.BP_SphereMoviePlayer_C"))
  (set `self.MoviePlayer` (`KismetArrayLibrary.Array_Get` _outactors))
  (`self.SetupUD360`) ; Default Play type
)

(event `self.ReceiveTick`
  (params (DeltaSeconds :type "Float (single-precision)"))
  ;[1 1 1] Movie Sphere moving with camera
  (`SceneComponent.K2_SetWorldLocation` (`self.Sphere`) (`SceneComponent.K2_GetComponentLocation` (`self.Camera`)) false false))

(event `Key|MotionController_Left_Trigger`
  (params (Key :type "Key Structure" :default "AnyKey"))
  (bind _widgetinteraction (`self.WidgetInteraction`))
  ;[1 1 1] Interaction Setting
  (:`Pressed`
    (`WidgetInteractionComponent.PressPointerKey` _widgetinteraction "LeftMouseButton" :!label _label))
  (:`Released`
    (`WidgetInteractionComponent.ReleasePointerKey` _widgetinteraction "LeftMouseButton" :!label _label_2)))

(event `Key|LeftMouseButton`
  (params (Key :type "Key Structure" :default "AnyKey"))
  ;[1 1 1] Interaction Setting
  (:`Pressed`
    (goto _label))
  (:`Released`
    (goto _label_2)))

(event `Key|MotionController_Right_Trigger`
  (params (Key :type "Key Structure" :default "AnyKey"))
  ;[1 1 1] Interaction Setting
  (:`Pressed`
    (goto _label))
  (:`Released`
    (goto _label_2)))

(event `SetupS180`
  (bind _sphere (`self.Sphere`))
  ;[1 1 1] Single 180
  (`PrimitiveComponent.SetMaterial` _sphere 0 "/Game/_Game/Materials/Mat_SingleMovie.Mat_SingleMovie")
  (`StaticMeshComponent.SetStaticMesh` _sphere "/Game/_Game/Meshs/SM_HalfSphere.SM_HalfSphere")
  (`SceneComponent.K2_SetWorldRotation` _sphere (struct :`Yaw` 180.0) false false))

(event `SetupS360`
  (bind _sphere (`self.Sphere`))
  ;[1 1 1] Single 360
  (`PrimitiveComponent.SetMaterial` _sphere 0 "/Game/_Game/Materials/Mat_SingleMovie.Mat_SingleMovie")
  (`StaticMeshComponent.SetStaticMesh` _sphere "/Game/_Game/Meshs/SM_Sphere.SM_Sphere")
  (`SceneComponent.K2_SetWorldRotation` _sphere (struct :`Yaw` 270.0) false false))

(event `SetupUD180`
  (bind _sphere (`self.Sphere`))
  ;[1 1 1] Up-Down 180
  (`PrimitiveComponent.SetMaterial` _sphere 0 "/Game/_Game/Materials/Mat_UpDownMovie.Mat_UpDownMovie")
  (`StaticMeshComponent.SetStaticMesh` _sphere "/Game/_Game/Meshs/SM_HalfSphere.SM_HalfSphere")
  (`SceneComponent.K2_SetWorldRotation` _sphere (struct :`Yaw` 180.0) false false))

(event `SetupUD360`
  (bind _sphere (`self.Sphere`))
  ;[1 1 1] Up-Down 360
  (`PrimitiveComponent.SetMaterial` _sphere 0 "/Game/_Game/Materials/Mat_UpDownMovie.Mat_UpDownMovie")
  (`StaticMeshComponent.SetStaticMesh` _sphere "/Game/_Game/Meshs/SM_Sphere.SM_Sphere")
  (`SceneComponent.K2_SetWorldRotation` _sphere (struct :`Yaw` 270.0) false false))

(event `SetupLR180`
  (bind _sphere (`self.Sphere`))
  ;[1 1 1] Left-Right 180
  (`PrimitiveComponent.SetMaterial` _sphere 0 "/Game/_Game/Materials/Mat_LeftRightMovie.Mat_LeftRightMovie")
  (`StaticMeshComponent.SetStaticMesh` _sphere "/Game/_Game/Meshs/SM_HalfSphere.SM_HalfSphere")
  (`SceneComponent.K2_SetWorldRotation` _sphere (struct :`Yaw` 180.0) false false))

(event `SetupLR360`
  (bind _sphere (`self.Sphere`))
  ;[1 1 1] Left-Right 360
  (`PrimitiveComponent.SetMaterial` _sphere 0 "/Game/_Game/Materials/Mat_LeftRightMovie.Mat_LeftRightMovie")
  (`StaticMeshComponent.SetStaticMesh` _sphere "/Game/_Game/Meshs/SM_Sphere.SM_Sphere")
  (`SceneComponent.K2_SetWorldRotation` _sphere (struct :`Yaw` 270.0) false false))

(fn `CheckMotionController`
  (bind _motioncontrollerright (`self.MotionControllerRight`))
  (bind _motioncontrollerleft (`self.MotionControllerLeft`))
  (bind _widgetinteraction (`self.WidgetInteraction`))
  (if (`MotionControllerComponent.IsTracked` _motioncontrollerright)
    (`SceneComponent.K2_AttachToComponent` _widgetinteraction _motioncontrollerright "None" "SnapToTarget" "SnapToTarget" "KeepRelative" true)
    (elif (`MotionControllerComponent.IsTracked` _motioncontrollerleft)
      (`SceneComponent.K2_AttachToComponent` _widgetinteraction _motioncontrollerleft "None" "SnapToTarget" "SnapToTarget" "KeepRelative" true))))

(fn `UserConstructionScript`)